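; BP_ZombChar is a zombie player character that runs forward automatically, jumps and collects brains for score.
; Tick feeds constant movement input along world X, scaled by Speed.
; Jump input triggers a jump and holds an IsJumping flag for a fixed one-second delay rather than detecting landing.
; BeginPlay creates the HUD widget, and AddBrain adds to PlayerScore and updates its brain counter text.
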(event EventBeginPlay
  ;[1 1 1] HUD
  (bind _returnvalue (UserInterface|CreateWidget "/Game/Blueprints/HUD.HUD_C"))
  (bind _output_get (Variables|Default|SetHUD _returnvalue))
  (UserInterface|Viewport|AddtoViewport _output_get 0))

(event Collision|EventActorBeginOverlap
  (params (OtherActor :type Actor%20Object%20Reference)))

(event EventTick
  (params (DeltaSeconds :type Float%20%28single-precision%29))
  ;[1 1 1] Move Forward
  (Pawn|Input|AddMovementInput "1.000000, 0, 0" (Variables|Default|GetSpeed) false))

(event Input|ActionEvents|InputActionJump
  (params (Key :type Key%20Structure :default "None"))
  ;[1 1 1] Jumping
  (:Pressed
    (Character|Jump)
    (Variables|Default|SetIsJumping true)
    (Utilities|FlowControl|Delay 1.0)
    (Variables|Default|SetIsJumping false)))

(fn ConstructionScript)

(fn AddBrain
  (params (BrainScore :type Integer))
  (Variables|Default|SetPlayerScore (+ (Variables|Default|GetPlayerScore) BrainScore))
  (Rendering|Components|TextRender|SetText (Variables|/Game/Blueprints/HUD.HUD_C|GetBrainsValue (Variables|Default|GetHUD)) (Utilities|Text|ToText(Integer) (Variables|Default|GetPlayerScore))))