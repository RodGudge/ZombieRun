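; Level piece actor that chains procedurally generated track for the zombie character (BP_ZombChar).
; When the character overlaps CollisionBox, it spawns a random class from the Levels array at the ArrowEnd transform, then destroys itself after a delay.
; A second Box trigger acts as game over, reloading the current level by name when the character touches it.
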(event OnComponentBeginOverlap(CollisionBox)
  (params (OverlappedComponent :type Primitive%20Component%20Object%20Reference) (OtherActor :type Actor%20Object%20Reference) (OtherComp :type Primitive%20Component%20Object%20Reference) (OtherBodyIndex :type Integer) (bFromSweep :type Boolean) (SweepResult :type Hit%20Result%20Structure%20%28by%20ref%29))
  (bind _levels (Variables|Default|GetLevels))
  ;[1 1 1] Spawn Level Piece
  (Utilities|Casting|CastToBP_ZombChar OtherActor)
  (Game|SpawnActorfromClass (Utilities|Array|Get(acopy) _levels (Math|Random|RandomIntegerinRange 0 (Utilities|Array|LastIndex _levels))) (Transformation|GetWorldTransform (Variables|Default|GetArrowEnd)) "Undefined" 0 0)
  ;[1 1 1] Remove Old Level Piece
  (Utilities|FlowControl|Delay 1e+01)
  (Actor|DestroyActor))

(event OnComponentBeginOverlap(Box)
  (params (OverlappedComponent :type Primitive%20Component%20Object%20Reference) (OtherActor :type Actor%20Object%20Reference) (OtherComp :type Primitive%20Component%20Object%20Reference) (OtherBodyIndex :type Integer) (bFromSweep :type Boolean) (SweepResult :type Hit%20Result%20Structure%20%28by%20ref%29))
  ;[1 1 1] Game Over (Restart Game)
  (Utilities|Casting|CastToBP_ZombChar OtherActor)
  (bind _returnvalue (Game|GetCurrentLevelName true))
  (Game|OpenLevel(byName) (Utilities|String|StringToName _returnvalue)))

(fn ConstructionScript)